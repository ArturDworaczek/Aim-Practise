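; Player Blueprint for the FPS, handling interaction prompt display, reload HUD feedback and weapon recoil.
; Spawn and remove events create the Interact_Widget on the viewport and take it down.
; ReloadAnim casts to MainHUD and starts or stops its reload animation through an inverted StopAnimation flag.
; KnockbackStart plays a timeline that nudges the gun mesh along local X each update, then snaps it back to a hardcoded rest position.
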(event EventSpawnInteraction
  (bind _returnvalue (UserInterface|CreateWidget "/Game/FPS_TR/Blueprints/Widgets/Interact_Widget.Interact_Widget_C" (Game|GetPlayerController 0)))
  (bind _output_get (Variables|Default|SetInteractionWidget _returnvalue))
  (UserInterface|Viewport|AddtoViewport _output_get 0))

(event EventRemoveInteraction
  (bind _interactionwidget (Variables|Default|GetInteractionWidget))
  (Utilities|IsValid _interactionwidget
    (:Is%20Valid
      (Widget|RemovefromParent _interactionwidget))))

(event EventReloadAnim
  (params (bStopAnimation :type Boolean))
  (bind _asmain_hud (Utilities|Casting|CastToMainHUD (HUD|GetHUD (Game|GetPlayerController 0))))
  (if bStopAnimation
    (Default|ReloadAnimation (Variables|/Game/FPS_TR/Gamemode/MainHUD.MainHUD_C|GetHUD _asmain_hud) false)
    (else
      (Default|ReloadAnimation (Variables|/Game/FPS_TR/Gamemode/MainHUD.MainHUD_C|GetHUD _asmain_hud) true))))

(event EventKnockbackStart
  (bind _gunmesh (Variables|Default|GetGunMesh))
  (bind _knockbackamount (Timeline|KnockbackTL PlayFromStart)
    (:Update
      (Transformation|AddRelativeLocation _gunmesh (Math|Vector|MakeVector _knockbackamount 0.0 0.0) true false))
    (:Finished
      (Transformation|SetRelativeLocation _gunmesh (Math|Vector|MakeVector 19.000004 25.0 -21.0) true false))))

(fn ConstructionScript)