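; Player controller for the FPS game mode that opens the pause menu and records action key bindings.
; On begin play it calls GetActionKeys, whose body is not in this file.
; The PauseMenu input spawns a MenuUI widget, switches to UI-only input and shows the cursor.
; The UpdateActionKey event adds received key information to ActionMappings on MainGameInstance_BP.
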(event EventBeginPlay
  ;[1 1 1] BeginPlay
  (Class|MainPlayerController|GetActionKeys))

(event EventUpdateActionKey
  (params (ActionKeyInformation :type Input%20Action%20Key%20Mapping%20Structure))
  ;[1 1 1] ActionKeys
  (bind _asmain_game_instance_bp (Utilities|Casting|CastToMainGameInstance_BP (Game|GetGameInstance)))
  (Utilities|Array|Add (Variables|/Game/FPS_TR/Gamemode/MainGameInstance_BP.MainGameInstance_BP_C|GetActionMappings _asmain_game_instance_bp) ActionKeyInformation))

(event Input|ActionEvents|InputActionPauseMenu
  (params (Key :type Key%20Structure))
  ;[1 1 1] Show PauseMenu
  (:Pressed
    (bind _returnvalue (UserInterface|CreateWidget "/Game/FPS_TR/Blueprints/Widgets/PauseMenu/MenuUI.MenuUI_C" self))
    (bind _output_get (Variables|Default|SetPauseMenu _returnvalue))
    (UserInterface|Viewport|AddtoViewport _output_get 99)
    (Input|SetInputModeUIOnly self _output_get "DoNotLock")
    (Variables|Default|SetbShowMouseCursor true)))

(fn ConstructionScript)